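; Tracker bot Blueprint that shows health changes on four WBP_BotHealthDelta widgets.
; On BeginPlay it finds all widgets of that class, nested ones included, and caches the first four by array index, with no count check.
; Its BotShowUI event forwards the health change and does-damage values to each cached widget's UpdateHealthText, so all four receive the same update.
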(event `self.ReceiveBeginPlay`
  (bind _foundwidgets (`WidgetBlueprintLibrary.GetAllWidgetsOfClass` "/Game/UI/WBP_BotHealthDelta.WBP_BotHealthDelta_C" false))
  (`|ExecutionSequence`
    (:`then_0`
      (set `self.Wall Widget Holder` (`|GetArrayItem` _foundwidgets)))
    (:`then_1`
      (set `self.Wall Widget Holder 2` (`|GetArrayItem` _foundwidgets 1)))
    (:`then_2`
      (set `self.Wall Widget Holder 3` (`|GetArrayItem` _foundwidgets 2)))
    (:`then_3`
      (set `self.Wall Widget Holder 4 ` (`|GetArrayItem` _foundwidgets 3)))))

(event `self.BotShowUI`
  (params (HealthCng :type "Float (single-precision)") (BDoesDamage :type Boolean))
  (`|ExecutionSequence`
    (:`then_0`
      (`/Game/UI/WBP_BotHealthDelta.Update Health text` (`self.Wall Widget Holder`) HealthCng BDoesDamage))
    (:`then_1`
      (`/Game/UI/WBP_BotHealthDelta.Update Health text` (`self.Wall Widget Holder 2`) HealthCng BDoesDamage))
    (:`then_2`
      (`/Game/UI/WBP_BotHealthDelta.Update Health text` (`self.Wall Widget Holder 3`) HealthCng BDoesDamage))
    (:`then_3`
      (`/Game/UI/WBP_BotHealthDelta.Update Health text` (`self.Wall Widget Holder 4 `) HealthCng BDoesDamage))))

(fn `UserConstructionScript`)